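; Spline-driven floor actor for the Boltworks environment that lays a floor mesh along an editable spline.
; The construction script measures the mesh's X length from its bounds and adds collidable spline mesh components at that interval along the spline.
; SetStartAndEnd bends each segment using local spline positions and tangents, clamping tangent size to the mesh length.
; All work happens at construction, with no active runtime events.
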(event EventBeginPlay)

(event Collision|EventActorBeginOverlap
  (params (OtherActor :type Actor%20Object%20Reference)))

(event EventTick
  (params (DeltaSeconds :type Float%20%28single-precision%29)))

(fn ConstructionScript
  (bind _spline_mesh (Variables|Default|GetSpline%20Mesh))
  (bind _returnvalue (StaticMesh|GetBoundingBox _spline_mesh))
  (Variables|Default|SetMeshForwardLength (.x (+ (Math|Vector|VectorGetAbs (.min _returnvalue)) (Math|Vector|VectorGetAbs (.max _returnvalue)))))
  (for _index (range 0 (Math|Float|Truncate (/ (Spline|GetSplineLength (Variables|Default|GetSpline)) (Variables|Default|GetMeshForwardLength))))
    (Variables|Default|SetCurrentIndex _index)
    (bind _returnvalue_2 (AddComponent|AddSplineMeshComponent false))
    (Utilities|FlowControl|Sequence
      (:then_0
        (Collision|SetCollisionEnabled _returnvalue_2 "QueryAndPhysics"))
      (:then_1
        (SplineMesh|SetForwardAxis _returnvalue_2 "X" true))
      (:then_2
        (Components|StaticMesh|SetStaticMesh _returnvalue_2 (Variables|Default|GetSpline%20Mesh)))
      (:then_3
        (CallFunction|SetStartandEnd _returnvalue_2)))))

(fn SetStartandEnd
  (params (Mesh%20Component :type Spline%20Mesh%20Component%20Object%20Reference))
  (bind _currentindex (Variables|Default|GetCurrentIndex))
  (bind _currentindex_2 (Variables|Default|GetCurrentIndex))
  (bind _meshforwardlength (Variables|Default|GetMeshForwardLength))
  (bind _meshforwardlength_2 (Variables|Default|GetMeshForwardLength))
  (bind _returnvalue (* _currentindex_2 _meshforwardlength))
  (bind _returnvalue_2 (+ _currentindex 1))
  (bind _returnvalue_3 (* _returnvalue_2 _meshforwardlength_2))
  (SplineMesh|SetStartandEnd Mesh%20Component (Spline|GetLocationatDistanceAlongSpline (Variables|Default|GetSpline) _returnvalue "Local") (Math|Vector|ClampVectorSize (Spline|GetTangentatDistanceAlongSpline (Variables|Default|GetSpline) _returnvalue "Local") 0.0 (Variables|Default|GetMeshForwardLength)) (Spline|GetLocationatDistanceAlongSpline (Variables|Default|GetSpline) _returnvalue_3 "Local") (Math|Vector|ClampVectorSize (Spline|GetTangentatDistanceAlongSpline (Variables|Default|GetSpline) _returnvalue_3 "Local") 0.0 (Variables|Default|GetMeshForwardLength)) true :!class /Script/Engine.SplineMeshComponent))